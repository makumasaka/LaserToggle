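; BP_Thing is an actor in the laser pointer feature that switches its visible shape between a sphere and a cube.
; BeginPlay shows the Sphere, hides the Cube and resets ThingState to zero.
; ToggleThing checks ThingState, swaps the hidden-in-game flags of the two components and flips the state, with no caller inside this Blueprint.
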(event `self.ReceiveBeginPlay`
  (`SceneComponent.SetHiddenInGame` (`self.Sphere`) false false)
  (`SceneComponent.SetHiddenInGame` (`self.Cube`) true false)
  (set `self.ThingState` 0.0))

(fn `ToggleThing`
  (if (== (`self.ThingState`) 0.0)
    (`SceneComponent.SetHiddenInGame` (`self.Sphere`) true false)
    (`SceneComponent.SetHiddenInGame` (`self.Cube`) false false)
    (set `self.ThingState` 1.0)
    (else
      (`SceneComponent.SetHiddenInGame` (`self.Sphere`) false false)
      (`SceneComponent.SetHiddenInGame` (`self.Cube`) true false)
      (set `self.ThingState` 0.0))))

(fn `UserConstructionScript`)